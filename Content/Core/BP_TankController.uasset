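; BP_TankController is the tank controller that drives the gameplay HUD.
; On BeginPlay it creates a WBP_GamePlayUI widget and adds it to the viewport.
; Every Tick it casts the controlled pawn to TankPawn, caches it, and pushes its HealthComponent's current and max health to the widget, polling rather than binding to events.
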(event EventBeginPlay
  (bind _returnvalue (UserInterface|CreateWidget "/Game/UI/MainHUD/WBP_GamePlayUI.WBP_GamePlayUI_C"))
  (bind _output_get (Variables|Default|SetGamePlayUI _returnvalue))
  (UserInterface|Viewport|AddtoViewport _output_get 0))

(event EventTick
  (params (DeltaSeconds :type Float%20%28single-precision%29))
  (bind _astank_pawn (Utilities|Casting|CastToTankPawn (Pawn|GetControlledPawn)))
  (bind _output_get (Variables|Default|SetMyTankPawn _astank_pawn))
  (Default|UpdateHealth (Variables|Default|GetGamePlayUI) (Variables|/Script/TankoGeddon.HealthComponent|GetCurrentHealth (Variables|/Script/TankoGeddon.MachinePawn|GetHealthComponent _output_get)) (Variables|/Script/TankoGeddon.HealthComponent|GetMaxHealth (Variables|/Script/TankoGeddon.MachinePawn|GetHealthComponent _output_get))))

(fn ConstructionScript)